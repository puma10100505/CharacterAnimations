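; Player controller that routes input actions for aiming, firing, crouching, weapon drop and pickup to the controlled BP_BasicLocoCharacter.
; Each press casts the controlled pawn, and the aim, fire and crouch releases reuse that cast result.
; Aiming and crouching require an equipped character, and aiming also lowers walk speed until release.
; Drop acts on the current weapon and pickup on the nearest one, each only when valid.
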(event `InputAction|Aiming`
  (params (Key :type "Key Structure"))
  ;[1 1 1] Aiming State
  (:`Pressed`
    (bind _asbp_basic_loco_character (cast `/Game/BasicLocomotion/Blueprints/BP_BasicLocoCharacter` (`self.K2_GetPawn`)))
    (if (`/Game/BasicLocomotion/Blueprints/BP_BasicLocoCharacter.bIsEquipped` _asbp_basic_loco_character)
      (set `/Game/BasicLocomotion/Blueprints/BP_BasicLocoCharacter.bIsAiming` true _asbp_basic_loco_character)
      (bind _charactermovement (`Character.CharacterMovement` _asbp_basic_loco_character))
      (set `CharacterMovementComponent.MaxWalkSpeed` 300.0 _charactermovement)))
  (:`Released`
    (set `/Game/BasicLocomotion/Blueprints/BP_BasicLocoCharacter.bIsAiming` false _asbp_basic_loco_character)
    (set `CharacterMovementComponent.MaxWalkSpeed` 600.0 _charactermovement)))

(event `InputAction|Fire`
  (params (Key :type "Key Structure"))
  ;[1 1 1] Fire State
  (:`Pressed`
    (bind _asbp_basic_loco_character (cast `/Game/BasicLocomotion/Blueprints/BP_BasicLocoCharacter` (`self.K2_GetPawn`)))
    (`/Game/BasicLocomotion/Blueprints/BP_BasicLocoCharacter.StartFire` _asbp_basic_loco_character))
  (:`Released`
    (`/Game/BasicLocomotion/Blueprints/BP_BasicLocoCharacter.StopFire` _asbp_basic_loco_character)))

(event `InputAction|Crouch`
  (params (Key :type "Key Structure"))
  (:`Pressed`
    (bind _asbp_basic_loco_character (cast `/Game/BasicLocomotion/Blueprints/BP_BasicLocoCharacter` (`self.K2_GetPawn`)))
    (if (`/Game/BasicLocomotion/Blueprints/BP_BasicLocoCharacter.bIsEquipped` _asbp_basic_loco_character)
      (if (`Character.CanCrouch` _asbp_basic_loco_character)
        (`Character.Crouch` _asbp_basic_loco_character))))
  (:`Released`
    (if (`Character.bIsCrouched` _asbp_basic_loco_character)
      (`Character.UnCrouch` _asbp_basic_loco_character))))

(event `InputAction|Drop`
  (params (Key :type "Key Structure"))
  (:`Pressed`
    (bind _asbp_basic_loco_character (cast `/Game/BasicLocomotion/Blueprints/BP_BasicLocoCharacter` (`self.K2_GetPawn`)))
    (bind _outweapon (`/Game/BasicLocomotion/Blueprints/BP_BasicLocoCharacter.GetCurrentWeapon` _asbp_basic_loco_character))
    (`/Engine/EditorBlueprintResources/StandardMacros.IsValid` _outweapon
      (:`Is Valid`
        (`/Game/BasicLocomotion/Blueprints/BP_BasicLocoCharacter.DropWeapon` _asbp_basic_loco_character _outweapon)))))

(event `InputAction|Pickup`
  (params (Key :type "Key Structure"))
  (:`Pressed`
    (bind _asbp_basic_loco_character (cast `/Game/BasicLocomotion/Blueprints/BP_BasicLocoCharacter` (`self.K2_GetPawn`)))
    (bind _nearestweapon (`/Game/BasicLocomotion/Blueprints/BP_BasicLocoCharacter.NearestWeapon` _asbp_basic_loco_character))
    (`/Engine/EditorBlueprintResources/StandardMacros.IsValid` _nearestweapon
      (:`Is Valid`
        (`/Game/BasicLocomotion/Blueprints/BP_BasicLocoCharacter.Pickup` _asbp_basic_loco_character _nearestweapon)))))

(fn `UserConstructionScript`)