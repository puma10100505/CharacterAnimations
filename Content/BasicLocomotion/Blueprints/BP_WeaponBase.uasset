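; BP_WeaponBase is the base weapon actor that a BP_BasicLocoCharacter picks up by walking into it.
; When PickupArea overlaps that character, the weapon registers itself through AddWeapon, turns off the pickup collision and stops physics simulation on WeaponMesh.
; If the character has nothing equipped, it also calls EquipWeapon and stores the index returned by AddWeapon as CurrentWeaponIndex.
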(event `self.PickupArea.OnComponentBeginOverlap`
  (params (OverlappedComponent :type "PrimitiveComponent Object Reference") (OtherActor :type "Actor Object Reference") (OtherComp :type "PrimitiveComponent Object Reference") (OtherBodyIndex :type Integer) (bFromSweep :type Boolean) (SweepResult :type "HitResult Structure (by ref)"))
  (bind _asbp_basic_loco_character (cast `/Game/BasicLocomotion/Blueprints/BP_BasicLocoCharacter` OtherActor))
  (bind _returnvalue (`/Game/BasicLocomotion/Blueprints/BP_BasicLocoCharacter.AddWeapon` _asbp_basic_loco_character self))
  (`PrimitiveComponent.SetCollisionEnabled` (`self.PickupArea`) "NoCollision")
  (`PrimitiveComponent.SetSimulatePhysics` (`self.WeaponMesh`) false)
  (if (not (`/Game/BasicLocomotion/Blueprints/BP_BasicLocoCharacter.bIsEquipped` _asbp_basic_loco_character))
    (`/Game/BasicLocomotion/Blueprints/BP_BasicLocoCharacter.EquipWeapon` _asbp_basic_loco_character self)
    (set `/Game/BasicLocomotion/Blueprints/BP_BasicLocoCharacter.CurrentWeaponIndex` _returnvalue _asbp_basic_loco_character)))

(fn `UserConstructionScript`)