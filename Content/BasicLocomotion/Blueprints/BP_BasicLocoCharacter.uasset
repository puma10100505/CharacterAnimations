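; Character Blueprint that manages a weapon inventory with pickup, equip, unequip, drop and firing.
; Equipping snaps the weapon to a hand or mount socket on the mesh and toggles between controller-yaw strafing and orient-to-movement rotation.
; Pickup auto-equips when nothing is held, while dropping detaches the weapon, re-enables its pickup area and throws it forward with physics.
; Fire calls forward to the weapon at the current list index.
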(fn `AddWeapon`
  (params (InNewWeapon :type "/Game/BasicLocomotion/Blueprints/BP_WeaponBase Object Reference"))
  (returns (ReturnValue :type Integer))
  (bind _returnvalue (`KismetArrayLibrary.Array_Add` (`self.WeaponList`) InNewWeapon))
  (`self.SetOwner` InNewWeapon self)
  (set `/Game/BasicLocomotion/Blueprints/BP_WeaponBase.OwnerPawn` self InNewWeapon)
  (return _returnvalue))

(fn `DropWeapon`
  (params (InWeapon :type "/Game/BasicLocomotion/Blueprints/BP_WeaponBase Object Reference"))
  (locals (TmpCurrentWeapon :type "/Game/BasicLocomotion/Blueprints/BP_WeaponBase Object Reference"))
  (if (== InWeapon (`self.GetCurrentWeapon`))
    (`self.UnequipWeapon` InWeapon)
    (`self.RemoveWeapon` InWeapon)
    (else
      (`self.RemoveWeapon` InWeapon)))
  (`self.K2_DetachFromActor` InWeapon "KeepWorld" "KeepWorld" "KeepWorld")
  (`PrimitiveComponent.SetCollisionEnabled` (`/Game/BasicLocomotion/Blueprints/BP_WeaponBase.PickupArea` InWeapon) "QueryOnly")
  (`PrimitiveComponent.SetSimulatePhysics` (`/Game/BasicLocomotion/Blueprints/BP_WeaponBase.WeaponMesh` InWeapon) true)
  (`PrimitiveComponent.AddForce` (`/Game/BasicLocomotion/Blueprints/BP_WeaponBase.WeaponMesh` InWeapon) (* (`self.GetActorForwardVector`) (`self.DropPower`)) "None" true))

(fn `EquipWeapon`
  (params (InEquipWeapon :type "/Game/BasicLocomotion/Blueprints/BP_WeaponBase Object Reference"))
  (`self.K2_AttachToComponent` InEquipWeapon (`self.Mesh`) (`/Game/BasicLocomotion/Blueprints/BP_WeaponBase.EquipSocket` InEquipWeapon) "SnapToTarget" "SnapToTarget" "SnapToTarget" true)
  (set `self.bIsEquipped` true)
  (set `self.bUseControllerRotationYaw` true)
  (set `CharacterMovementComponent.bOrientRotationToMovement` false (`self.CharacterMovement`))
  (set `CameraComponent.bUsePawnControlRotation` true (`self.FollowCamera`))
  (set `self.CurrentWeaponIndex` (`KismetArrayLibrary.Array_Find` (`self.WeaponList`) InEquipWeapon)))

(fn `GetCurrentWeapon`
  (returns (OutWeapon :type "/Game/BasicLocomotion/Blueprints/BP_WeaponBase Object Reference"))
  (if (== (`self.CurrentWeaponIndex`) -1)
    (return null)
    (else
      (return (`|GetArrayItem` (`self.WeaponList`) (`self.CurrentWeaponIndex`))))))

(fn `Pickup`
  (params (InWeapon :type "/Game/BasicLocomotion/Blueprints/BP_WeaponBase Object Reference"))
  (bind _returnvalue (`self.AddWeapon` InWeapon))
  (`PrimitiveComponent.SetCollisionEnabled` (`/Game/BasicLocomotion/Blueprints/BP_WeaponBase.PickupArea` InWeapon) "NoCollision")
  (`PrimitiveComponent.SetSimulatePhysics` (`/Game/BasicLocomotion/Blueprints/BP_WeaponBase.WeaponMesh` InWeapon) false)
  (if (not (`self.bIsEquipped`))
    (`self.EquipWeapon` InWeapon)
    (set `self.CurrentWeaponIndex` _returnvalue)))

(fn `RemoveWeapon`
  (params (InWeapon :type "/Game/BasicLocomotion/Blueprints/BP_WeaponBase Object Reference"))
  (bind _returnvalue (`KismetArrayLibrary.Array_Find` (`self.WeaponList`) InWeapon))
  (if (not (== _returnvalue -1))
    (`KismetArrayLibrary.Array_Remove` (`self.WeaponList`) _returnvalue)
    (`self.SetOwner` InWeapon null)
    (set `/Game/BasicLocomotion/Blueprints/BP_WeaponBase.OwnerPawn` null InWeapon)))

(fn `StartFire`
  (locals (CurrentWeapon :type "/Game/BasicLocomotion/Blueprints/BP_WeaponBase Object Reference"))
  (bind _outweapon (`self.GetCurrentWeapon`))
  (`/Engine/EditorBlueprintResources/StandardMacros.IsValid` _outweapon
    (:`Is Valid`
      (bind _output_get (set `local.CurrentWeapon` _outweapon))
      (`/Game/BasicLocomotion/Blueprints/BP_WeaponBase.StartFire` _output_get))))

(fn `StopFire`
  (locals (CurrentWeapon :type "/Game/BasicLocomotion/Blueprints/BP_WeaponBase Object Reference"))
  (bind _outweapon (`self.GetCurrentWeapon`))
  (`/Engine/EditorBlueprintResources/StandardMacros.IsValid` _outweapon
    (:`Is Valid`
      (bind _output_get (set `local.CurrentWeapon` _outweapon))
      (`/Game/BasicLocomotion/Blueprints/BP_WeaponBase.StopFire` _output_get))))

(fn `UnequipWeapon`
  (params (InWeapon :type "/Game/BasicLocomotion/Blueprints/BP_WeaponBase Object Reference"))
  (`self.K2_AttachToComponent` InWeapon (`self.Mesh`) (`/Game/BasicLocomotion/Blueprints/BP_WeaponBase.MountSocket` InWeapon) "SnapToTarget" "SnapToTarget" "SnapToTarget" true)
  (set `self.bIsEquipped` false)
  (set `self.bUseControllerRotationYaw` false)
  (set `CharacterMovementComponent.bOrientRotationToMovement` true (`self.CharacterMovement`))
  (set `CameraComponent.bUsePawnControlRotation` false (`self.FollowCamera`))
  (set `self.CurrentWeaponIndex` -1))

(fn `UserConstructionScript`)